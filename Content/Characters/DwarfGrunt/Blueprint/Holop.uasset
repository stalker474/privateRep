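; Holop is a dwarf grunt character Blueprint with attachable weapon and armor, an overhead stats widget and a paper sprite.
; The construction script applies both attachments and sets itself as the pawn on the StatsOverhead widget.
; If that cast succeeds, it also adds the sprite to the show-only list of the first SceneCapture2D found in the level.
; The event graph holds only an empty Tick.
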(event EventTick
  (params (DeltaSeconds :type Float%20%28single-precision%29)))

(fn ConstructionScript
  (Class|StrategyChar|SetWeaponAttachment (Variables|Default|GetWeaponAttachmentBlueprint))
  (Class|StrategyChar|SetArmorAttachment (Variables|Default|GetArmorAttachmentBlueprint))
  (bind _asstats_overhead (Utilities|Casting|CastToStatsOverhead (UserInterface|GetUserWidgetObject (Variables|Default|GetWidget))))
  (Variables|/Game/UI/HUD/StatsOverhead.StatsOverhead_C|SetPawn _asstats_overhead self)
  (bind _outactors (Actor|GetAllActorsOfClass "/Script/Engine.SceneCapture2D"))
  (Rendering|SceneCapture|ShowOnlyComponent (Variables|/Script/Engine.SceneCapture2D|GetCaptureComponent2D (Utilities|Array|Get(acopy) _outactors)) (Variables|Default|GetPaperSprite)))