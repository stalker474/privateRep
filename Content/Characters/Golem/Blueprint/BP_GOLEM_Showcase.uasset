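; Showcase Blueprint that demonstrates a golem constructing itself, roaring, idling, then dying by exploding.
; It uses two meshes: a skinned golem for roar and idle, and a split-piece golem for the construct and explode animations.
; BeginPlay runs the whole one-shot sequence, toggling visibility to swap meshes and using fixed delays timed to the animations rather than completion events.
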(event EventBeginPlay
  ;[1 1 1] SHOWCASE PURPOSE ONLY: example of how to make the golem appear by constructing itself and dying by exploding
  (Rendering|SetVisibility (Variables|SkeletalMeshActor|GetSkeletalMeshComponent) false false) ; hide the skinned version of the Golem
  (Components|Animation|PlayAnimation (Variables|SkeletalMeshActor|GetSkeletalMeshComponent) "/Game/Characters/Golem/Animations/GOLEM_idle.GOLEM_idle" true) ; Skinned Version Plays Idle Animation
  (Components|Animation|PlayAnimation (Variables|Default|GetGOLEM_SPLIT_idle) "/Game/Characters/Golem/Animations/GOLEM_SPLIT_idle_Anim.GOLEM_SPLIT_idle_Anim" true) ; Split Version plays Idle Animation
  (Components|Animation|PlayAnimation (Variables|Default|GetGOLEM_SPLIT_idle) "/Game/Characters/Golem/Animations/GOLEM_SPLIT_construct_Anim.GOLEM_SPLIT_construct_Anim" false) ; Split Version Construct itself by playing construct animation
  (Utilities|FlowControl|Delay 7.5) ; Time to wait till construct animation is finished playing
  (Components|Animation|PlayAnimation (Variables|SkeletalMeshActor|GetSkeletalMeshComponent) "/Game/Characters/Golem/Animations/GOLEM_roar.GOLEM_roar" false) ; tells Skinned version the to perform the ROAR animation
  (Rendering|SetVisibility (Variables|SkeletalMeshActor|GetSkeletalMeshComponent) true false) ; Unhide Skinned Version
  (Rendering|SetVisibility (Variables|Default|GetGOLEM_SPLIT_idle) false false) ; Hide Split version
  (Utilities|FlowControl|Delay 2.5) ; Time to wait till ROAr animation is finished
  (Components|Animation|PlayAnimation (Variables|SkeletalMeshActor|GetSkeletalMeshComponent) "/Game/Characters/Golem/Animations/GOLEM_idle.GOLEM_idle" true) ; Tells Skinned Version to Perform IDLE animation loop
  (Utilities|FlowControl|Delay 6.0) ; time to wait before exploding the golem
  (Rendering|SetVisibility (Variables|SkeletalMeshActor|GetSkeletalMeshComponent) false false) ; Hide Skinned Version Of Golem
  (Rendering|SetVisibility (Variables|Default|GetGOLEM_SPLIT_idle) true false) ; Unhide Split Version of Golem
  (Components|Animation|PlayAnimation (Variables|Default|GetGOLEM_SPLIT_idle) "/Game/Characters/Golem/Animations/GOLEM_SPLIT_explode_Anim.GOLEM_SPLIT_explode_Anim" false) ; Make Split gorlm performs the EXPLODe animation
)

(event EventActorBeginOverlap
  (params (OtherActor :type Actor%20Object%20Reference)))

(event EventTick
  (params (DeltaSeconds :type Float%20%28single-precision%29)))

(fn ConstructionScript)