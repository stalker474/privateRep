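; Default tower building Blueprint with an overhead stats widget and a team-dependent ground target decal.
; The construction script and BeginPlay both assign the tower as the Pawn of its StatsOverhead widget.
; Every tick it compares its team with that of the first player's MobaTestCharacter and sets the decal to the standard material for the same team or the enemy material otherwise.
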(event EventBeginPlay
  (bind _asstats_overhead (Utilities|Casting|CastToStatsOverhead (UserInterface|GetUserWidgetObject (Variables|Default|GetWidget))))
  (Variables|/Game/UI/HUD/StatsOverhead.StatsOverhead_C|SetPawn _asstats_overhead self))

(event Collision|EventActorBeginOverlap
  (params (OtherActor :type Actor%20Object%20Reference)))

(event EventTick
  (params (DeltaSeconds :type Float%20%28single-precision%29))
  (bind _returnvalue (Game|GetPlayerController 0))
  (bind _decalcomponent (Variables|Default|GetDecalComponent))
  (bind _returnvalue_2 (Pawn|GetControlledPawn _returnvalue))
  (Utilities|IsValid _returnvalue
    (:Is%20Valid
      (Utilities|IsValid _returnvalue_2
        (:Is%20Valid
          (bind _asmoba_test_character (Utilities|Casting|CastToMobaTestCharacter _returnvalue_2))
          (if (== (Class|StrategyBuilding|GetTeamNum) (Class|MobaTestCharacter|GetTeamNum _asmoba_test_character))
            (Rendering|Components|Decal|SetDecalMaterial _decalcomponent "/Game/UI/GroundTargetMaterial.GroundTargetMaterial")
            (else
              (Rendering|Components|Decal|SetDecalMaterial _decalcomponent "/Game/UI/GroundTargetMaterialEnnemy.GroundTargetMaterialEnnemy"))))))))

(fn ConstructionScript
  (bind _asstats_overhead (Utilities|Casting|CastToStatsOverhead (UserInterface|GetUserWidgetObject (Variables|Default|GetWidget))))
  (Variables|/Game/UI/HUD/StatsOverhead.StatsOverhead_C|SetPawn _asstats_overhead self))