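; Player spawn point actor that shows client-side team and player-name visuals, apparently for a lobby.
; On BeginPlay, non-authority instances reveal either the Blue or Red component according to the spawn's team number.
; PlayerChanged, also handled only on remote instances, writes the new name into the PlayerNameLobby widget held by the Name component.
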(event EventBeginPlay
  (bind _blue (Variables|Default|GetBlue))
  (bind _red (Variables|Default|GetRed))
  (Networking|SwitchHasAuthority
    (:Remote
      (switch Utilities|FlowControl|Switch|SwitchonEStrategyTeam (Utilities|Enum|ByteToEnumEStrategyTeam (Class|StrategySpawnPoint|GetTeamNum))
        (:Blue
          (Utilities|IsValid _blue
            (:Is%20Valid
              (Rendering|SetVisibility _blue true false))))
        (:Red
          (Utilities|IsValid _red
            (:Is%20Valid
              (Rendering|SetVisibility _red true false))))))))

(event Collision|EventActorBeginOverlap
  (params (OtherActor :type Actor%20Object%20Reference)))

(event EventTick
  (params (DeltaSeconds :type Float%20%28single-precision%29)))

(event EventPlayerChanged
  (params (Name :type String))
  (Networking|SwitchHasAuthority
    (:Remote
      (bind _asplayer_name_lobby (Utilities|Casting|CastToPlayerNameLobby (UserInterface|GetUserWidgetObject (Variables|Default|GetName))))
      (Rendering|Components|TextRender|SetText (Variables|/Game/UI/HUD/PlayerNameLobby.PlayerNameLobby_C|GetTextBlock_Name _asplayer_name_lobby) (Utilities|Text|ToText(String) Name)))))

(fn ConstructionScript)